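; FlashingMonster is a monster that strikes its AI controller's target once that target is inside its AttackRange.
; Tick either counts down the reload after a shot or checks AttackRange overlaps for the MonsterController's MyTarget and calls the server fire event.
; Firing spawns a FlashingMonsterStrike at the target's transform and starts the reload.
; Each shot shortens the next reload by a fixed step, with no lower limit.
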(event `self.ReceiveTick`
  (params (DeltaSeconds :type "Float (single-precision)"))
  (if (`self.bIsRecoiling`)
    (bind _output_get (set `self.CurrentReloadTime` (- (`self.CurrentReloadTime`) DeltaSeconds)))
    (set `self.bIsRecoiling` (> _output_get 0.0))
    (else
      (bind _asmonster_controller (cast `MonsterController` (`self.GetController`)))
      (if (!= (`KismetArrayLibrary.Array_Find` (`PrimitiveComponent.GetOverlappingActors` (`self.AttackRange`) null) (`MonsterController.MyTarget` _asmonster_controller)) -1)
        (`self.Server_Fire`)))))

(event `Server_Fire`
  (bind _maxreloadtime (`self.MaxReloadTime`))
  (bind _asmonster_controller (cast `MonsterController` (`self.GetController`)))
  (`|SpawnActorFromClass` "/Game/Projectiles/Blueprints/FlashingMonsterStrike.FlashingMonsterStrike_C" (`self.GetTransform` (`MonsterController.MyTarget` _asmonster_controller)) "Undefined" "OverrideRootScale" self self)
  (set `self.bIsRecoiling` true)
  (set `self.CurrentReloadTime` _maxreloadtime)
  (set `self.MaxReloadTime` (- _maxreloadtime 0.2)))

(fn `UserConstructionScript`)