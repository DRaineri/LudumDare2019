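; Monster that explodes when an FPV or TDV character enters its detection volume, then destroys itself.
; A larger ExplosionRadius component maintains a list of overlapping actors on the authority only.
; Exploding calls ServerLoseLife for a fixed amount on each FPV or TDV character in that list.
; The detection trigger itself has no authority check.
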(event `self.ExplosionDetection.OnComponentBeginOverlap`
  (params (OverlappedComponent :type "PrimitiveComponent Object Reference") (OtherActor :type "Actor Object Reference") (OtherComp :type "PrimitiveComponent Object Reference") (OtherBodyIndex :type Integer) (bFromSweep :type Boolean) (SweepResult :type "HitResult Structure (by ref)"))
  (cast `FPVCharacter` OtherActor
    (:`then`
      _)
    (:`CastFailed`
      (cast `TDVCharacter` OtherActor)))
  (`self.Explode`)
  (`self.K2_DestroyActor`))

(event `Explode`
  (for _array_element (`self.ActorsInRangeForExplosion`)
    (bind _astdvcharacter (cast `TDVCharacter` _array_element)
      (:`then`
        (`TDVCharacter.Server_LoseLife` _astdvcharacter 20.0))
      (:`CastFailed`
        (bind _asfpvcharacter (cast `FPVCharacter` _array_element))
        (`FPVCharacter.Server_LoseLife` _asfpvcharacter 20.0)))))

(event `self.ExplosionRadius.OnComponentBeginOverlap`
  (params (OverlappedComponent :type "PrimitiveComponent Object Reference") (OtherActor :type "Actor Object Reference") (OtherComp :type "PrimitiveComponent Object Reference") (OtherBodyIndex :type Integer) (bFromSweep :type Boolean) (SweepResult :type "HitResult Structure (by ref)"))
  (bind _actorsinrangeforexplosion (`self.ActorsInRangeForExplosion`))
  (`/Engine/EditorBlueprintResources/ActorMacros.Switch Has Authority`
    (:`Authority`
      (if (== (`KismetArrayLibrary.Array_Find` _actorsinrangeforexplosion OtherActor) -1)
        (`KismetArrayLibrary.Array_Add` _actorsinrangeforexplosion OtherActor)))))

(event `self.ExplosionRadius.OnComponentEndOverlap`
  (params (OverlappedComponent :type "PrimitiveComponent Object Reference") (OtherActor :type "Actor Object Reference") (OtherComp :type "PrimitiveComponent Object Reference") (OtherBodyIndex :type Integer))
  (bind _actorsinrangeforexplosion (`self.ActorsInRangeForExplosion`))
  (`/Engine/EditorBlueprintResources/ActorMacros.Switch Has Authority`
    (:`Authority`
      (if (!= (`KismetArrayLibrary.Array_Find` _actorsinrangeforexplosion OtherActor) -1)
        (`KismetArrayLibrary.Array_RemoveItem` _actorsinrangeforexplosion OtherActor)))))

(fn `UserConstructionScript`)