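; BP_MyGameInstance is a Game Instance Blueprint that handles hosting and ending a multiplayer session.
; HostGame shows a loading screen and creates a four-connection session, with LAN use set by EnableLan.
; On success it opens FirstPersonExampleMap as a listen server and sets game-only input; on failure it shows an error dialog.
; DestroySession tears the session down for the first player controller.
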(event `self.HostGame`
  (`self.ShowLoadingScreen`)
  (`CreateSessionCallbackProxy.CreateSession` (`GameplayStatics.GetPlayerController` 0) 4 (`self.EnableLan`)
    (:`OnSuccess`
      (`GameplayStatics.OpenLevel` "FirstPersonExampleMap" true "listen")
      (`WidgetBlueprintLibrary.SetInputMode_GameOnly` (`GameplayStatics.GetPlayerController` 0)))
    (:`OnFailure`
      (`self.ShowErrorDialog` "Fail create session"))))

(event `self.DestroySession`
  (`DestroySessionCallbackProxy.DestroySession` (`GameplayStatics.GetPlayerController` 0)))